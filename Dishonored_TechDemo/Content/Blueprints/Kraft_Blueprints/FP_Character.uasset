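; First-person player character with crouch and three powers resembling Dishonored's: Darkvision, Blink and Windblast.
; Darkvision toggles a detection sphere and material parameter collection, revealing overlapped AI_Darkvision vision cones and custom-depth meshes.
; Holding Blink adjusts a spring arm's length from camera pitch on Tick; releasing plays an FOV timeline and teleports to BlinkTarget.
; Windblast applies an impulse along a control-rotation line trace; crouch repeats a capsule trace while it hits.
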(event `self.ReceiveTick`
  (params (DeltaSeconds :type "Float (single-precision)"))
  (if (`self.isUsingBlink`)
    (`self.BlinkDistanceDetermination`)))

(event `InputAction|Crouch`
  (params (Key :type "Key Structure"))
  (bind _capsulecomponent (`self.CapsuleComponent`))
  ;[1 1 1] Crouch
  (:`Pressed`
    (`self.Crouch`)
    (bind (_outhit _returnvalue) (`KismetSystemLibrary.CapsuleTraceSingle` :`Start` (`SceneComponent.K2_GetComponentLocation` _capsulecomponent) :`End` (+ (* (`SceneComponent.GetForwardVector` (`self.FirstPersonCamera`)) (`SceneComponent.GetForwardVector` (`self.CapsuleComponent`))) (0.0 0.0 0.1)) :`Radius` (`CapsuleComponent.CapsuleRadius` _capsulecomponent) :`HalfHeight` (`CapsuleComponent.CapsuleHalfHeight` _capsulecomponent) :`TraceChannel` "TraceTypeQuery1" :`DrawDebugType` "Persistent" :!label _label))
    (bind _output_get (set `self.crouchHit?` _returnvalue))
    (if _output_get
      (set `self.Half Height Adjust` 25.0)
      (`KismetSystemLibrary.Delay` 0.01)
      (goto _label)))
  (:`Released`
    (`self.UnCrouch`)
    (set `self.crouchHit?` false)))

(event `self.ReceiveBeginPlay`
  (`parent.ReceiveBeginPlay`)
  (`|ExecutionSequence`))

(event `InputAction|Activate Darkvision`
  (params (Key :type "Key Structure"))
  (bind _darkvisionradius (`self.DarkvisionRadius`))
  ;[1 1 1] Darkvision
  (:`Pressed`
    (`KismetSystemLibrary.Delay` 0.2) ; Add in delay for animation later
    (if (`self.isUsingDarkvision`)
      (`KismetMaterialLibrary.SetScalarParameterValue` "/Game/Materials/Kraft_Materials/DarkvisionParameter.DarkvisionParameter" "RadiusOpacity")
      (`SphereComponent.SetSphereRadius` _darkvisionradius 0.0 true)
      (set `self.isUsingDarkvision` false)
      (else
        (`KismetMaterialLibrary.SetScalarParameterValue` "/Game/Materials/Kraft_Materials/DarkvisionParameter.DarkvisionParameter" "RadiusOpacity" 1.0)
        (set `self.isUsingDarkvision` true)
        (`SphereComponent.SetSphereRadius` _darkvisionradius 600.0 true)))))

(event `self.DarkvisionRadius.OnComponentBeginOverlap`
  (params (OverlappedComponent :type "PrimitiveComponent Object Reference") (OtherActor :type "Actor Object Reference") (OtherComp :type "PrimitiveComponent Object Reference") (OtherBodyIndex :type Integer) (bFromSweep :type Boolean) (SweepResult :type "HitResult Structure (by ref)"))
  ;[1 1 1] Darkvision
  (if (`self.isUsingDarkvision`)
    (bind _asai_darkvision (cast `/Game/Blueprints/Kraft_Blueprints/AI_Darkvision` OtherActor))
    (`SceneComponent.SetVisibility` (`/Game/Blueprints/Kraft_Blueprints/AI_Darkvision.VisionCone` _asai_darkvision) true false)
    (`PrimitiveComponent.SetRenderCustomDepth` (`Character.Mesh` _asai_darkvision) true)
    (`KismetMaterialLibrary.SetScalarParameterValue` "/Game/Materials/Kraft_Materials/DarkvisionParameter.DarkvisionParameter" "Opacity" 1.0)))

(event `self.DarkvisionRadius.OnComponentEndOverlap`
  (params (OverlappedComponent :type "PrimitiveComponent Object Reference") (OtherActor :type "Actor Object Reference") (OtherComp :type "PrimitiveComponent Object Reference") (OtherBodyIndex :type Integer))
  ;[1 1 1] Darkvision
  (if (`self.isUsingDarkvision`)
    (bind _asai_darkvision (cast `/Game/Blueprints/Kraft_Blueprints/AI_Darkvision` OtherActor))
    (bind _visioncone (`/Game/Blueprints/Kraft_Blueprints/AI_Darkvision.VisionCone` _asai_darkvision))
    (`SceneComponent.SetVisibility` _visioncone false false)
    (`PrimitiveComponent.SetRenderCustomDepth` _visioncone false)
    (`PrimitiveComponent.SetRenderCustomDepth` (`Character.Mesh` _asai_darkvision) false)
    (`KismetMaterialLibrary.SetScalarParameterValue` "/Game/Materials/Kraft_Materials/DarkvisionParameter.DarkvisionParameter" "Opacity")))

(event `InputAction|Activate Blink`
  (params (Key :type "Key Structure"))
  (bind _firstpersoncamera (`self.FirstPersonCamera`))
  ;[1 1 1] Blink
  (:`Pressed`
    ;;[1 1 1] Aiming blink makes final location visible
    (set `self.isUsingBlink` true)
    (`PrimitiveComponent.SetMaterial` (`self.FirstPersonMesh`) 0 "/Game/LevelPrototyping/Materials/MI_Solid_Blue.MI_Solid_Blue")
    (`SceneComponent.SetVisibility` (`self.Niagara`) true false))
  (:`Released`
    (`PrimitiveComponent.SetMaterial` (`self.FirstPersonMesh`) 0 "/Game/FirstPersonArms/Character/Materials/M_UE4Man_Body.M_UE4Man_Body")
    (`SceneComponent.SetVisibility` (`self.Niagara`) false false)
    (`self.BlinkDistanceDetermination`)
    (bind (_outhit _returnvalue) (`KismetSystemLibrary.LineTraceSingle` :`Start` (`SceneComponent.K2_GetComponentLocation` _firstpersoncamera) :`End` (+ (* (`SceneComponent.GetForwardVector` _firstpersoncamera) (`KismetMathLibrary.Conv_DoubleToVector` 8000.0)) (0.0 0.0 0.0)) :`TraceChannel` "TraceTypeQuery1" :`DrawDebugType` "ForDuration"))
    (if _returnvalue
      _
      (else
        _))
    (`|ExecutionSequence`
      (:`then_0`
        ;;[1 1 1] Animation
        (bind (_direction _blinkfov_change) (`Timeline|Timeline` :!via `PlayFromStart`)
          (:`Update`
            (`CameraComponent.SetFieldOfView` (`self.FirstPersonCamera`) _blinkfov_change))))
      (:`then_1`
        (`KismetSystemLibrary.Delay` 0.15)
        (`self.K2_SetActorLocation` (`SceneComponent.K2_GetComponentLocation` (`self.BlinkTarget`)) false true)
        (set `self.isUsingBlink` false)))))

(event `BlinkDistanceDetermination`
  (bind _blinkdistance (`self.BlinkDistance`))
  ;[1 1 1] Blink
  ;;[1 1 1] Depending on the vertical direction you look while aiming blink, the overall distance is affected.
  (bind _output_get (set `SpringArmComponent.TargetArmLength` (`SpringArmComponent.TargetArmLength` _blinkdistance) _blinkdistance))
  (bind _output_get_2 (set `self.camUpVector` (`SceneComponent.GetUpVector` (`self.FirstPersonCamera`))))
  (set `SpringArmComponent.TargetArmLength` (`KismetMathLibrary.FClamp` (+ (* (.z _output_get_2) _output_get) 100.0) 450.0 1000.0) (`self.BlinkDistance`)))

(event `InputAction|Activate Windblast`
  (params (Key :type "Key Structure"))
  (bind _returnvalue (`self.K2_GetActorLocation`))
  ;[1 1 1] Activate Windblast
  (:`Pressed`
    (bind _outhit (`KismetSystemLibrary.LineTraceSingle` _returnvalue (+ _returnvalue (* (`KismetMathLibrary.GetForwardVector` (`self.GetControlRotation`)) (`KismetMathLibrary.Conv_DoubleToVector` 15000.0))) "TraceTypeQuery1"))
    (`PrimitiveComponent.AddImpulse` (`.HitComponent` (`GameplayStatics.BreakHitResult` _outhit)) (* (`KismetMathLibrary.GetForwardVector` (`self.GetControlRotation`)) (`KismetMathLibrary.Conv_DoubleToVector` 1500.0)) "None" true)
    (`AddComponent|NODE_AddNiagaraComponent-0` :`RelativeTransform` (`SceneComponent.GetRelativeTransform` (`self.FirstPersonCamera`)))
    (`ActorComponent.SetActive` (`self.Niagara`) false false)))

(fn `UserConstructionScript`
  (`parent.UserConstructionScript`))