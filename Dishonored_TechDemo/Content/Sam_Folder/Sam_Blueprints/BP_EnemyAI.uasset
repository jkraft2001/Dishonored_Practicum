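; BP_EnemyAI is an enemy that chases the player character once its PawnSensing component sees a pawn.
; A sighting sets IsSeeingPlayer, which is never cleared here, and calls FollowPlayer, which prints a debug string and runs AIMoveTo toward player 0.
; On arrival it only clears CanAttack if set; the file has no attack action or reset for that flag.
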(event `self.PawnSensing.OnSeePawn`
  (params (Pawn :type "Pawn Object Reference"))
  (set `self.isSeeingPlayer` true)
  (`self.FollowPlayer`))

(event `FollowPlayer`
  (if (`self.isSeeingPlayer`)
    (`KismetSystemLibrary.PrintString` "Is Seeing Character")
    (`|AIMoveTo` self (0.0 0.0 0.0) (`GameplayStatics.GetPlayerCharacter` 0) 20.0
      (:`OnSuccess`
        (if (`self.CanAttack`)
          (set `self.CanAttack` false))))))

(fn `UserConstructionScript`)