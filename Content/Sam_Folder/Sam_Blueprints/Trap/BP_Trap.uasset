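; BP_Trap is a single-use trap that detonates when an enemy (BP_EnemyAI) overlaps its Box trigger.
; On trigger it fires a RadialForce impulse and applies radial damage with falloff around the Trap component.
; It then prints a debug message, hides the Trap component and destroys itself after a short delay.
; A player-overlap branch and a sparks emitter spawn remain in the graph but never run.
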(event `self.Box.OnComponentBeginOverlap`
  (params (OverlappedComponent :type "PrimitiveComponent Object Reference") (OtherActor :type "Actor Object Reference") (OtherComp :type "PrimitiveComponent Object Reference") (OtherBodyIndex :type Integer) (bFromSweep :type Boolean) (SweepResult :type "HitResult Structure (by ref)"))
  (`|ExecutionSequence`
    (:`then_0`
      (cast `/Game/Sam_Folder/Sam_Blueprints/BP_EnemyAI` OtherActor)
      (`RadialForceComponent.FireImpulse` (`self.RadialForce`))
      (`GameplayStatics.ApplyRadialDamageWithFalloff` :`BaseDamage` (`self.Base Damage`) :`MinimumDamage` 5.0 :`Origin` (`SceneComponent.K2_GetComponentLocation` (`self.Trap`)) :`DamageInnerRadius` 50.0 :`DamageOuterRadius` 100.0 :`DamageFalloff` 2.0 :`DamageCauser` self :`InstigatedByController` null)
      (`KismetSystemLibrary.PrintString` "Damaged enemy")
      (`SceneComponent.SetHiddenInGame` (`self.Trap`) true false)
      (`KismetSystemLibrary.Delay` 1.0)
      (`self.K2_DestroyActor`))))

(fn `UserConstructionScript`)