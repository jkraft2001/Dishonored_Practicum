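; Enemy AI Blueprint that detects pawns by sight, chases them on command and damages the player on contact.
; PawnSensing starts a detection message on the seen pawn once, and a retriggerable delay stops it and resets the DoOnce when sightings lapse.
; StartChase and StopChase toggle the flag gating AIMoveTo toward the seen pawn, with stop also halting movement.
; Any capsule overlap applies fixed damage to the first player character, whatever actor overlapped.
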(event `self.PawnSensing.OnSeePawn`
  (params (Pawn :type "Pawn Object Reference"))
  ;[1 1 1] Enemy Detect Player
  (`|ExecutionSequence`
    (:`then_0`
      (`|ExecutionSequence`
        (:`then_0`
          (`/Engine/EditorBlueprintResources/StandardMacros.DoOnce` false :!label _label
            (:`Completed`
              (message `/Game/Sam_Folder/Sam_Blueprints/DetectionMeter/BP_DetectionInterface.StartDetection` Pawn self))))
        (:`then_1`
          (if (`self.ShouldChase?`)
            (`|AIMoveTo` self (0.0 0.0 0.0) Pawn)))))
    (:`then_1`
      (`KismetSystemLibrary.RetriggerableDelay` 0.5)
      (message `/Game/Sam_Folder/Sam_Blueprints/DetectionMeter/BP_DetectionInterface.StopDetection` Pawn)
      (goto _label :!via `Reset`))))

(event `/Game/Sam_Folder/Sam_Blueprints/DetectionMeter/BP_DetectionInterface.StartChase`
  ;[1 1 1] Enemy Start and Stop Chasing Player
  (set `self.ShouldChase?` true))

(event `/Game/Sam_Folder/Sam_Blueprints/DetectionMeter/BP_DetectionInterface.StopChase`
  ;[1 1 1] Enemy Start and Stop Chasing Player
  (set `self.ShouldChase?` false)
  (`MovementComponent.StopMovementImmediately` (`self.CharacterMovement`)))

(event `self.CapsuleCollision.OnComponentBeginOverlap`
  (params (OverlappedComponent :type "PrimitiveComponent Object Reference") (OtherActor :type "Actor Object Reference") (OtherComp :type "PrimitiveComponent Object Reference") (OtherBodyIndex :type Integer) (bFromSweep :type Boolean) (SweepResult :type "HitResult Structure (by ref)"))
  ;[1 1 1] Dealing Damage to Player
  (`GameplayStatics.ApplyDamage` (`GameplayStatics.GetPlayerCharacter` 0) 5.0))

(fn `UserConstructionScript`)