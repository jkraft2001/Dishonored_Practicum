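; BP_Grenade is a timed grenade that primes itself on BeginPlay and explodes after a short fuse.
; When the fuse ends it activates ForceComp, whose activation event drives the whole detonation.
; That event spawns explosion particles and sound, fires a physics impulse, and applies radial damage with falloff at the mesh location.
; It then hides the mesh and destroys the actor after a brief delay.
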(event `self.ReceiveBeginPlay`
  (`self.OnPrimed`))

(event `OnPrimed`
  (`KismetSystemLibrary.Delay` 4.0)
  (`ActorComponent.Activate` (`self.ForceComp`) false))

(event `self.ForceComp.OnComponentActivated`
  (params (Component :type "ActorComponent Object Reference") (bReset :type Boolean))
  (bind _meshcomp (`self.MeshComp`))
  (bind _returnvalue (`SceneComponent.K2_GetComponentLocation` _meshcomp))
  (`GameplayStatics.SpawnEmitterAtLocation` "/Game/StarterContent/Particles/P_Explosion.P_Explosion" _returnvalue (`SceneComponent.K2_GetComponentRotation` _meshcomp))
  (`GameplayStatics.PlaySoundAtLocation` "/Game/StarterContent/Audio/Explosion_Cue.Explosion_Cue" _returnvalue (struct) 1.0 1.0 0.0 null null null null)
  (`RadialForceComponent.FireImpulse` (`self.ForceComp`))
  (`GameplayStatics.ApplyRadialDamageWithFalloff` :`BaseDamage` 50.0 :`MinimumDamage` 5.0 :`Origin` (`SceneComponent.K2_GetComponentLocation` (`self.MeshComp`)) :`DamageInnerRadius` 100.0 :`DamageOuterRadius` 200.0 :`DamageFalloff` 2.0 :`DamageCauser` self :`InstigatedByController` null :`DamagePreventionChannel` "ECC_WorldStatic")
  (`SceneComponent.SetHiddenInGame` (`self.MeshComp`) true false)
  (`KismetSystemLibrary.Delay` 3.0)
  (`self.K2_DestroyActor`))

(fn `UserConstructionScript`)