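; Trigger volume that lets a crouched FP_Character hide by shrinking its capsule and lowering its eye height below the normal crouch values.
; The player reference is cached on BeginPlay, and the box responds only to that player's SizeDet component rather than the whole character.
; Overlap events set the player's CrouchHit flag, then recheck it after a short delay before applying or restoring crouch proportions, only while crouched.
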(event `self.ReceiveBeginPlay`
  ;[1 1 1] Gets a refrence to player character
  (bind _outactors (`GameplayStatics.GetAllActorsOfClass` "/Game/Blueprints/Kraft_Blueprints/FP_Character.FP_Character_C"))
  (set `self.RefToPlayer` (`|GetArrayItem` _outactors)) ; promoted variable of get copy(0) of FP Character
)

(event `self.Box.OnComponentBeginOverlap`
  (params (OverlappedComponent :type "PrimitiveComponent Object Reference") (OtherActor :type "Actor Object Reference") (OtherComp :type "PrimitiveComponent Object Reference") (OtherBodyIndex :type Integer) (bFromSweep :type Boolean) (SweepResult :type "HitResult Structure (by ref)"))
  (bind _reftoplayer (`self.RefToPlayer`))
  ;[1 1 1] When the player overlaps the crouch trigger, capsule proportions are adjusted so they can hide.
  (if (== OtherComp (`/Game/Blueprints/Kraft_Blueprints/FP_Character.SizeDet` _reftoplayer))
    (bind _output_get (set `/Game/Blueprints/Kraft_Blueprints/FP_Character.crouchHit?` true _reftoplayer))
    (`KismetSystemLibrary.Delay` 0.1)
    (if _output_get
      (if (`/Game/Blueprints/Kraft_Blueprints/FP_Character.crouched?` _reftoplayer)
        (`CapsuleComponent.SetCapsuleSize` (`Character.CapsuleComponent` _reftoplayer) (`self.lowerCrouchCapsuleRadius`) (`self.lowerCrouchCapsuleHeight`) true)
        (set `Pawn.BaseEyeHeight` 16.0 _reftoplayer)))))

(event `self.Box.OnComponentEndOverlap`
  (params (OverlappedComponent :type "PrimitiveComponent Object Reference") (OtherActor :type "Actor Object Reference") (OtherComp :type "PrimitiveComponent Object Reference") (OtherBodyIndex :type Integer))
  (bind _reftoplayer (`self.RefToPlayer`))
  ;[1 1 1] When the player leaves, while still crouched, the capsule proportions return to normal.
  (if (== OtherComp (`/Game/Blueprints/Kraft_Blueprints/FP_Character.SizeDet` _reftoplayer))
    (bind _output_get (set `/Game/Blueprints/Kraft_Blueprints/FP_Character.crouchHit?` false _reftoplayer))
    (`KismetSystemLibrary.Delay` 0.1)
    (if _output_get
      _
      (elif (`/Game/Blueprints/Kraft_Blueprints/FP_Character.crouched?` _reftoplayer)
        (`CapsuleComponent.SetCapsuleSize` (`Character.CapsuleComponent` _reftoplayer) (`self.crouchCapsuleRadius`) (`self.crouchCapsuleHeight`) true)
        (set `Pawn.BaseEyeHeight` 32.0 _reftoplayer)))))

(fn `UserConstructionScript`)