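; BP_RatPawn is a rat pawn that wanders at random and damages actors that touch it.
; From BeginPlay, Move sends it through AI MoveTo to a random reachable point near its current location, then repeats after a short random delay.
; The loop continues only on a successful move, which also prints a debug string.
; Capsule overlap applies a small fixed damage to the other actor, with no filtering.
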(event `self.ReceiveBeginPlay`
  (`self.Move`))

(event `self.ReceiveTick`
  (params (DeltaSeconds :type "Float (single-precision)")))

(event `Move`
  (`|AIMoveTo` self (`NavigationSystemV1.K2_GetRandomReachablePointInRadius` (`self.K2_GetActorLocation`) 500.0 null null) null
    (:`OnSuccess`
      (`KismetSystemLibrary.PrintString` "Hello")
      (`KismetSystemLibrary.Delay` (`KismetMathLibrary.RandomFloatInRange` 1.0 3.0))
      (`self.Move`))))

(event `self.Capsule.OnComponentBeginOverlap`
  (params (OverlappedComponent :type "PrimitiveComponent Object Reference") (OtherActor :type "Actor Object Reference") (OtherComp :type "PrimitiveComponent Object Reference") (OtherBodyIndex :type Integer) (bFromSweep :type Boolean) (SweepResult :type "HitResult Structure (by ref)"))
  (`GameplayStatics.ApplyDamage` OtherActor 1.0))

(fn `UserConstructionScript`)