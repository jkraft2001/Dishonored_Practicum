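; Rat pawn that wanders at random until enough nearby rats form a swarm that hunts characters.
; A group sphere counts overlapping rats to toggle swarm eligibility, switching between recursive Move and Swarm AIMoveTo loops.
; Player-spawned swarms target the first AI_Darkvision found; others chase the nearer of it or the player.
; Swarming rats damage what their capsule overlaps and destroy the AI shortly after a move toward it ends, even if failed.
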(event `self.ReceiveBeginPlay`
  ;[0.8691 0.2554 1] BeginPlay. Gather reference to the AI and the players within a level instance. Start movement.
  (bind _outactors (`GameplayStatics.GetAllActorsOfClass` "/Game/Blueprints/Kraft_Blueprints/AI_Blueprints/AI_Darkvision.AI_Darkvision_C"))
  (set `self.RefToAI` (`|GetArrayItem` _outactors))
  (bind _outactors_2 (`GameplayStatics.GetAllActorsOfClass` "/Game/Blueprints/Kraft_Blueprints/FP_Character.FP_Character_C"))
  (set `self.RefToPlayer` (`|GetArrayItem` _outactors_2))
  (set `self.Health` 2.0)
  (if (`self.bIsSwarmEligible?`)
    (`self.Swarm`)
    (else
      (`self.Move`))))

(event `Swarm`
  (bind _returnvalue (`self.K2_GetActorLocation`))
  (bind _returnvalue_2 (`self.K2_GetActorLocation` (`self.RefToAI`)))
  (bind _returnvalue_3 (`self.K2_GetActorLocation` (`self.RefToPlayer`)))
  ;[0 1 0.01835] Swarm. If the player spawns the rats (via the Rat Swarm IA() ), rats will move towards closest AI. If the rats are not spawned by the player and eligible for a swarm, they will move towards the closest Pawn actor between the player and the AI.
  (if (`self.bIsSwarmEligible?`)
    (if (`self.bIsPlayerSpawned?`)
      (`|AIMoveTo` self _returnvalue_2 null 2.0 :!label _label
        (:`OnSuccess`
          _)
        (:`OnFail`
          _))
      (if (`self.bIsSwarmEligible?`)
        (`KismetSystemLibrary.Delay` 2.0)
        (if (`self.bIsSwarmEligible?`)
          (`self.K2_DestroyActor` (`self.RefToAI`))
          (`self.Swarm` :!label _label_2)
          (else
            (`self.Move` :!label _label_3)))
        (else
          (goto _label_3)))
      (elif (> (`KismetMathLibrary.Vector_Distance` _returnvalue_2 _returnvalue) (`KismetMathLibrary.Vector_Distance` _returnvalue_3 _returnvalue))
        (`|AIMoveTo` self _returnvalue_3 null 2.0
          (:`OnSuccess`
            _)
          (:`OnFail`
            _))
        (if (`self.bIsSwarmEligible?`)
          (goto _label_2)
          (else
            (goto _label_3)))
        (else
          (goto _label))))
    (else
      (`self.Move`))))

(event `Move`
  ;[0 1 0.01835] Move. If a swarm is ineligible, rats will randomly patrol. If a swarm is ever eligible, their movement will change to a Swarm().
  (if (`self.bIsSwarmEligible?`)
    (`self.Swarm`)
    (else
      (`|AIMoveTo` null (`NavigationSystemV1.K2_GetRandomReachablePointInRadius` (`self.K2_GetActorLocation`) 500.0 null null) null 15.0
        (:`OnSuccess`
          (`KismetSystemLibrary.Delay` (`KismetMathLibrary.RandomFloatInRange` 3.0 5.0))
          (if (`self.bIsSwarmEligible?`)
            (`self.Swarm`)
            (else
              (`self.Move`))))
        (:`OnFail`
          (if (`self.bIsSwarmEligible?`)
            (`self.Swarm`)
            (else
              (`self.Move`))))))))

(event `self.GroupSphere.OnComponentBeginOverlap`
  (params (OverlappedComponent :type "PrimitiveComponent Object Reference") (OtherActor :type "Actor Object Reference") (OtherComp :type "PrimitiveComponent Object Reference") (OtherBodyIndex :type Integer) (bFromSweep :type Boolean) (SweepResult :type "HitResult Structure (by ref)"))
  ;[1 0 0] Overlap with Sphere. Tracks all the rats in proximity to each other. If the total is >= 10, Swarm() is called. Else, Move(). Once the overlap is ended, check surroundings. If less than 10, Move(). Else, Swarm().
  (if (`ActorComponent.ComponentHasTag` OtherComp "Swarm")
    (bind _output_get (set `self.bIsSwarmEligible?` (>= (`KismetArrayLibrary.Array_LastIndex` (`self.GetOverlappingActors` OtherActor "BP_RatPawn_C")) 10)))
    (if _output_get
      (`self.Swarm`)
      (else
        (`self.Move`)))))

(event `self.GroupSphere.OnComponentEndOverlap`
  (params (OverlappedComponent :type "PrimitiveComponent Object Reference") (OtherActor :type "Actor Object Reference") (OtherComp :type "PrimitiveComponent Object Reference") (OtherBodyIndex :type Integer))
  ;[1 0 0] Overlap with Sphere. Tracks all the rats in proximity to each other. If the total is >= 10, Swarm() is called. Else, Move(). Once the overlap is ended, check surroundings. If less than 10, Move(). Else, Swarm().
  (if (< (`KismetArrayLibrary.Array_LastIndex` (`self.GetOverlappingActors` (stale `self.GroupSphere.OnComponentBeginOverlap` OtherActor) "BP_RatPawn_C")) 10)
    (set `self.bIsSwarmEligible?` false)
    (`self.Move`)
    (else
      (`self.Swarm`))))

(event `self.Capsule.OnComponentBeginOverlap`
  (params (OverlappedComponent :type "PrimitiveComponent Object Reference") (OtherActor :type "Actor Object Reference") (OtherComp :type "PrimitiveComponent Object Reference") (OtherBodyIndex :type Integer) (bFromSweep :type Boolean) (SweepResult :type "HitResult Structure (by ref)"))
  ;[1 0 0] Overlap with Capsule. Apply damage to actors only when a swarm is eligible.
  (if (or (`ActorComponent.ComponentHasTag` OtherComp "Rat") (`ActorComponent.ComponentHasTag` OtherComp "Swarm"))
    _
    (elif (`self.bIsSwarmEligible?`)
      (`GameplayStatics.ApplyDamage` OtherActor 1.0))))

(fn `UserConstructionScript`)