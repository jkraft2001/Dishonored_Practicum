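; BP_Clamber is a box volume that lets the player clamber onto a ledge during Blink.
; On overlap while Blink is active, it spawns a Niagara indicator at the BlinkTarget.
; If the overlapper is the player's SizeDet component, it raises max step height and, if Space is already held, teleports the player to the box's top center.
; End overlap restores step height and deactivates the indicator.
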(event `self.ReceiveBeginPlay`
  ;[1 1 1] Gets a refrence to player character
  (bind _outactors (`GameplayStatics.GetAllActorsOfClass` "/Game/Blueprints/Kraft_Blueprints/FP_Character.FP_Character_C"))
  (set `self.RefToPlayer` (`|GetArrayItem` _outactors)) ; promoted variable of get copy(0) of FP Character
)

(event `self.Box.OnComponentBeginOverlap`
  (params (OverlappedComponent :type "PrimitiveComponent Object Reference") (OtherActor :type "Actor Object Reference") (OtherComp :type "PrimitiveComponent Object Reference") (OtherBodyIndex :type Integer) (bFromSweep :type Boolean) (SweepResult :type "HitResult Structure (by ref)"))
  (bind _reftoplayer (`self.RefToPlayer`))
  (bind (_origin _boxextent) (`KismetSystemLibrary.GetComponentBounds` (`self.Box`)))
  (bind (_returnvalue_location _returnvalue_rotation _returnvalue_scale) (`KismetMathLibrary.BreakTransform` (`SceneComponent.GetRelativeTransform` (`/Game/Blueprints/Kraft_Blueprints/FP_Character.BlinkTarget` _reftoplayer))))
  ;[1 1 1] Change the VFX of the BlinkTarget to indicate potential clambering.
  (if (`/Game/Blueprints/Kraft_Blueprints/FP_Character.isUsingBlink` _reftoplayer)
    (bind _returnvalue (`NiagaraFunctionLibrary.SpawnSystemAtLocation` "/Game/Niagara/NewNiagaraSystem.NewNiagaraSystem" _returnvalue_location _returnvalue_rotation _returnvalue_scale))
    (bind _output_get (set `/Game/Blueprints/Kraft_Blueprints/FP_Character.BlinkTargetVFX` _returnvalue _reftoplayer))
    ;[1 1 1] While the player is in the volume, set their maximum step height to 180. If they press 'Space' while in the volume, they "clamber" to the top of volume.
    (if (== OtherComp (`/Game/Blueprints/Kraft_Blueprints/FP_Character.SizeDet` _reftoplayer))
      (set `CharacterMovementComponent.MaxStepHeight` 180.0 (`Character.CharacterMovement` _reftoplayer))
      (if (`PlayerController.IsInputKeyDown` (`GameplayStatics.GetPlayerController` 0) "SpaceBar")
        (`self.K2_SetActorLocation` _reftoplayer (+ _origin (`KismetMathLibrary.MakeVector` 0.0 0.0 (.z _boxextent))) false true) ; Set's actor location to top of the box volume, centered on the origin.
      ))
    (else
      (`ActorComponent.Deactivate` _output_get :!label _label))))

(event `self.Box.OnComponentEndOverlap`
  (params (OverlappedComponent :type "PrimitiveComponent Object Reference") (OtherActor :type "Actor Object Reference") (OtherComp :type "PrimitiveComponent Object Reference") (OtherBodyIndex :type Integer))
  ;[1 1 1] Change the VFX of the BlinkTarget to indicate potential clambering.
  (set `CharacterMovementComponent.MaxStepHeight` 45.0 (`Character.CharacterMovement` (`self.RefToPlayer`)))
  (goto _label))

(fn `UserConstructionScript`)