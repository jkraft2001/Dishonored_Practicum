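; First-person player character with Dishonored-style powers: blink, time bend, possession, darkvision, windblast and rat swarm, plus grenades, crouch and camera leaning.
; Input events gate most powers on mana and possession state, with upgrade flags strengthening several.
; Blink teleports to a spring-arm target scaled by view pitch, and darkvision reveals AI through an overlap sphere and custom depth.
; Possession fakes control by destroying the traced target, moving into its place and respawning its class on exit.
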(event `self.ReceiveTick`
  (params (DeltaSeconds :type "Float (single-precision)"))
  (`|ExecutionSequence`
    (:`then_0`
      (set `self.MaxHealth_0` (`KismetMathLibrary.FClamp` (`self.MaxHealth_0`) 0.0 100.0)))
    (:`then_1`
      (set `self.maxMana` (`KismetMathLibrary.FClamp` (`self.maxMana`) 0.0 100.0)))
    (:`then_2`
      (if (> (`self.maxMana`) 0.0)
        (set `self.hasMana` true)))
    (:`then_3`
      (if (`self.isUsingBlink`)
        (`self.BlinkDistanceDetermination`)))))

(event `InputAction|ThrowGrenade`
  (params (Key :type "Key Structure"))
  (:`Pressed`
    (bind _returnvalue (`|SpawnActorFromClass` "/Game/Blueprints/Kraft_Blueprints/BP_Grenade.BP_Grenade_C" (`KismetMathLibrary.MakeTransform` (+ (`SceneComponent.K2_GetComponentLocation` (`self.FirstPersonMesh`)) (0.0 0.0 25.0))) "Undefined" "MultiplyWithRoot" null null))
    (`/Game/Blueprints/Kraft_Blueprints/BP_Grenade.OnPrimed` _returnvalue)))

(event `self.ReceiveBeginPlay`
  (`parent.ReceiveBeginPlay`)
  (`|ExecutionSequence`
    (:`then_0`
      (set `self.MaxHealth_0` 100.0))
    (:`then_1`
      (set `self.maxMana` 100.0))
    (:`then_2`
      (set `self.maxSpeed` (`MovementComponent.GetMaxSpeed` (`self.CharacterMovement`))))))

(event `InputAction|Rat Swarm`
  (params (Key :type "Key Structure"))
  ;[0.3142 0.04208 0] Rat swarm
  (:`Pressed`
    (if (`self.hasMana`)
      (if (not (`self.Is Possessing?`))
        (`self.RatSwarm`)))))

(event `InputAction|Activate Darkvision`
  (params (Key :type "Key Structure"))
  (bind _darkvisionradius (`self.DarkvisionRadius`))
  ;[1 0.413 0.01319] Darkvision
  (:`Pressed`
    (if (`self.hasMana`)
      (if (not (`self.Is Possessing?`))
        (`KismetSystemLibrary.Delay` 0.2) ; Add in delay for animation later
        (if (`self.isUsingDarkvision`)
          (`KismetMaterialLibrary.SetScalarParameterValue` "/Game/Materials/Kraft_Materials/DarkvisionParameter.DarkvisionParameter" "RadiusOpacity")
          (`SphereComponent.SetSphereRadius` _darkvisionradius 0.0 true)
          (set `self.isUsingDarkvision` false)
          (else
            (`KismetMaterialLibrary.SetScalarParameterValue` "/Game/Materials/Kraft_Materials/DarkvisionParameter.DarkvisionParameter" "RadiusOpacity" 1.0)
            (set `self.isUsingDarkvision` true)
            (`SphereComponent.SetSphereRadius` _darkvisionradius 600.0 true)))))))

(event `InputAction|Activate Windblast`
  (params (Key :type "Key Structure"))
  ;[0.2622 0.3052 1] Activate Windblast
  (:`Pressed`
    (if (`self.hasMana`)
      (if (not (`self.Is Possessing?`))
        (`self.WindBlast`)))))

(event `self.DarkvisionRadius.OnComponentBeginOverlap`
  (params (OverlappedComponent :type "PrimitiveComponent Object Reference") (OtherActor :type "Actor Object Reference") (OtherComp :type "PrimitiveComponent Object Reference") (OtherBodyIndex :type Integer) (bFromSweep :type Boolean) (SweepResult :type "HitResult Structure (by ref)"))
  ;[1 0.413 0.01319] Darkvision
  (if (`self.isUsingDarkvision`)
    (bind _asai_darkvision (cast `/Game/Blueprints/Kraft_Blueprints/AI_Darkvision` OtherActor))
    (`SceneComponent.SetVisibility` (`/Game/Blueprints/Kraft_Blueprints/AI_Darkvision.VisionCone` _asai_darkvision) true false)
    (`PrimitiveComponent.SetRenderCustomDepth` (`Character.Mesh` _asai_darkvision) true)
    (`KismetMaterialLibrary.SetScalarParameterValue` "/Game/Materials/Kraft_Materials/DarkvisionParameter.DarkvisionParameter" "Opacity" 1.0)))

(event `InputAction|Stealth Lean Left`
  (params (Key :type "Key Structure"))
  ;[0.3906 0.3906 0.3906] Leaning
  (:`Pressed`
    (goto _label :!via `execute2`))
  (:`Released`
    (`self.LeanLeft` :!label _label)))

(event `self.DarkvisionRadius.OnComponentEndOverlap`
  (params (OverlappedComponent :type "PrimitiveComponent Object Reference") (OtherActor :type "Actor Object Reference") (OtherComp :type "PrimitiveComponent Object Reference") (OtherBodyIndex :type Integer))
  ;[1 0.413 0.01319] Darkvision
  (if (`self.isUsingDarkvision`)
    (bind _asai_darkvision (cast `/Game/Blueprints/Kraft_Blueprints/AI_Darkvision` OtherActor))
    (bind _visioncone (`/Game/Blueprints/Kraft_Blueprints/AI_Darkvision.VisionCone` _asai_darkvision))
    (`SceneComponent.SetVisibility` _visioncone false false)
    (`PrimitiveComponent.SetRenderCustomDepth` _visioncone false)
    (`PrimitiveComponent.SetRenderCustomDepth` (`Character.Mesh` _asai_darkvision) false)
    (`KismetMaterialLibrary.SetScalarParameterValue` "/Game/Materials/Kraft_Materials/DarkvisionParameter.DarkvisionParameter" "Opacity")))

(event `InputAction|Crouch`
  (params (Key :type "Key Structure"))
  ;[0.3906 0.3906 0.3906] Crouch
  (:`Pressed`
    (`/Engine/EditorBlueprintResources/StandardMacros.FlipFlop`
      (:`A`
        (`self.Crouch`)
        (set `self.crouched?` true))
      (:`B`
        (`self.UnCrouch`)
        (set `self.crouched?` false)))))

(event `InputAction|Stealth Lean Right`
  (params (Key :type "Key Structure"))
  ;[0.3906 0.3906 0.3906] Leaning
  (:`Pressed`
    (goto _label_2 :!via `execute2`))
  (:`Released`
    (`self.LeanRight` :!label _label_2)))

(event `InputAction|Activate Blink`
  (params (Key :type "Key Structure"))
  (bind _firstpersoncamera (`self.FirstPersonCamera`))
  ;[1 0.9569 0.3385] Blink
  (:`Pressed`
    (if (`self.hasMana`)
      (if (not (`self.Is Possessing?`))
        ;;[1 1 1] Aiming blink makes final location visible
        (set `self.isUsingBlink` true)
        (`PrimitiveComponent.SetMaterial` (`self.FirstPersonMesh`) 0 "/Game/LevelPrototyping/Materials/MI_Solid_Blue.MI_Solid_Blue")
        (bind _returnvalue (`NiagaraFunctionLibrary.SpawnSystemAtLocation` "/Game/BlinkAndDashVFX/VFX_Niagara/NS_Blink_Psionic.NS_Blink_Psionic" (`SceneComponent.K2_GetComponentLocation` (`self.BlinkTarget`)) (struct) (1.0 1.0 1.0) false false)) ; update location + make effect constant
      )))
  (:`Released`
    (if (`self.hasMana`)
      (if (not (`self.Is Possessing?`))
        (`PrimitiveComponent.SetMaterial` (`self.FirstPersonMesh`) 0 "/Game/FirstPersonArms/Character/Materials/M_UE4Man_Body.M_UE4Man_Body")
        (`ActorComponent.Deactivate` _returnvalue)
        (`self.BlinkDistanceDetermination`)
        (bind (_outhit _returnvalue_2) (`KismetSystemLibrary.LineTraceSingle` :`Start` (`SceneComponent.K2_GetComponentLocation` _firstpersoncamera) :`End` (+ (* (`SceneComponent.GetForwardVector` _firstpersoncamera) (`KismetMathLibrary.Conv_DoubleToVector` 8000.0)) (0.0 0.0 0.0)) :`TraceChannel` "TraceTypeQuery1" :`DrawDebugType` "ForDuration"))
        (if _returnvalue_2
          _
          (else
            _))
        (`|ExecutionSequence`
          (:`then_0`
            (`GameplayStatics.PlaySound2D` "/Game/Audio/blink_001.blink_001" 1.0 1.0 0.0 null null))
          (:`then_1`
            ;;[1 1 1] Animation
            (bind (_direction _blinkfov_change) (`Timeline|BlinkCam_Timeline` :!via `PlayFromStart`)
              (:`Update`
                (`CameraComponent.SetFieldOfView` (`self.FirstPersonCamera`) _blinkfov_change))))
          (:`then_2`
            (`KismetSystemLibrary.Delay` 0.15)
            (`self.BlinkDistanceDetermined`)))))))

(event `BlinkDistanceDetermination`
  (bind _blinkdistance (`self.BlinkDistance`))
  ;[1 0.9569 0.3385] Blink
  ;;[1 1 1] Depending on the vertical direction you look while aiming blink, the overall distance is affected.
  (bind _output_get (set `SpringArmComponent.TargetArmLength` (`SpringArmComponent.TargetArmLength` _blinkdistance) _blinkdistance))
  (bind _output_get_2 (set `self.camUpVector` (`SceneComponent.GetUpVector` (`self.FirstPersonCamera`))))
  (if (`self.bBlinkUpgrade`)
    (bind _returnvalue (+ (* (.z _output_get_2) _output_get) 100.0))
    (set `SpringArmComponent.TargetArmLength` (`KismetMathLibrary.FClamp` _returnvalue 600.0 1300.0) (`self.BlinkDistance`))
    (else
      (set `SpringArmComponent.TargetArmLength` (`KismetMathLibrary.FClamp` _returnvalue 450.0 1000.0) (`self.BlinkDistance`)))))

(event `InputAction|Activate Bend Time`
  (params (Key :type "Key Structure"))
  ;[0.3108 1 0.3417] Bend Time
  (:`Pressed`
    (if (`self.hasMana`)
      (if (`self.Is Possessing?`)
        _
        (elif (`self.timeBend`)
          ;;[1 1 1] On BeginPlay, BendTime is set to false. If pressed while true, revert time changes.
          (`GameplayStatics.SetGlobalTimeDilation` 1.0)
          (set `self.CustomTimeDilation` 1.0)
          (else
            (`|ExecutionSequence`
              (:`then_0`
                (`GameplayStatics.PlaySound2D` "/Game/Audio/timeBend_activate.timeBend_activate" 1.0 1.0 0.0 null null)
                ;;[1 1 1] Set TimeBend to true. Play animation and change view to grayscale.
                (set `self.timeBend` true)
                (`KismetSystemLibrary.Delay` 0.3) ; Delays the activation to sync up with audio
                (`GameplayStatics.PlaySound2D` "/Game/Audio/abilityActive.abilityActive" 1.0 1.0 0.0 null null) ; If ability is deactivated early, end sound. Idk how...
                ;;;[1 1 1] Set view to grayscale
                (`Timeline|Timeline` :!via `PlayFromStart`
                  (:`Update`
                    (`CameraComponent.SetPostProcessBlendWeight` (`self.FirstPersonCamera`) 0.0))))
              (:`then_1`
                (if (`self.bTimeBendUpgrade`)
                  ;;[1 1 1] Set time while true to slower. After a delay, set timeBend to false.
                  (`GameplayStatics.SetGlobalTimeDilation` 0.0)
                  (set `self.CustomTimeDilation` 5.0)
                  (`KismetSystemLibrary.Delay` 2.0)
                  (set `self.timeBend` false)
                  (else
                    ;;[1 1 1] Set time while true to slower. After a delay, set timeBend to false.
                    (`GameplayStatics.SetGlobalTimeDilation` 0.2)
                    (set `self.CustomTimeDilation` 5.0)
                    (`KismetSystemLibrary.Delay` 2.0)
                    (set `self.timeBend` false))))
              (:`then_2`
                ;;[1 1 1] Revert time changes if timeBend is set to false.
                (if (not (`self.timeBend`))
                  (`GameplayStatics.SetGlobalTimeDilation` 1.0)
                  (set `self.CustomTimeDilation` 1.0)
                  (`GameplayStatics.PlaySound2D` "/Game/Audio/timeBend_rampUp.timeBend_rampUp" 1.0 1.0 0.0 null null))))))))))

(event `InputAction|Possession`
  (params (Key :type "Key Structure"))
  ;[0 0.9967 1] Possession
  (:`Pressed`
    (bind _returnvalue (`NiagaraFunctionLibrary.SpawnSystemAtLocation` "/Game/VFX/NS_PossEffect.NS_PossEffect" (`SceneComponent.K2_GetComponentLocation` (`self.PossessionTarget`)))) ; update location
  )
  (:`Released`
    (if (`self.Is Possessing?`)
      (`self.Un Possess`)
      (elif (`self.hasMana`)
        (bind (_possessedpawn _bispossessing_ _pawncopy _output_get _output) (`self.Possess`))
        (`ActorComponent.Deactivate` _returnvalue)
        (set `self.Is Possessing?` _bispossessing_)
        (`KismetSystemLibrary.Delay` (`self.possDuration`)) ; if we are still posessing after 5 secondes, unposess
        (if (`self.Is Possessing?`)
          (`self.Un Possess`))))))

(event `Un Possess`
  ;[0 0.9967 1] Possession
  (set `self.Is Possessing?` false)
  (`|SpawnActorFromClass` (stale `InputAction|Possession` _pawncopy) (`KismetMathLibrary.MakeTransform` (+ (`self.K2_GetActorLocation` self) (`self.GetActorForwardVector` self)) (`self.K2_GetActorRotation` self)) "Undefined" "MultiplyWithRoot" null null)
  (`KismetArrayLibrary.Array_RemoveItem` (stale `InputAction|Possession` _output_get) (stale `InputAction|Possession` _output)))

(fn `BlinkDistanceDetermined`
  (`self.K2_SetActorLocation` (`SceneComponent.K2_GetComponentLocation` (`self.BlinkTarget`)) false true)
  (if (`self.bBlinkUpgrade`)
    (set `self.BlinkLengthDefault` 1300.0)
    (set `self.isUsingBlink` false)
    (else
      (set `SpringArmComponent.TargetArmLength` (`self.BlinkLengthDefault`) (`self.BlinkDistance`))
      (set `self.isUsingBlink` false))))

(fn `Possess`
  (returns (PossessedPawn :type "Actor Object Reference") (`bIsPossessing?` :type Boolean) (PawnCopy :type "Actor Class Reference") (Output_Get :type "Array of HitResult Structure") (Output :type "HitResult Structure"))
  (bind _returnvalue (`SceneComponent.K2_GetComponentLocation` (`self.FirstPersonCamera`)))
  (bind (_outhits _returnvalue_2) (`KismetSystemLibrary.LineTraceMultiForObjects` :`Start` _returnvalue :`End` (+ _returnvalue (* (`KismetMathLibrary.GetForwardVector` (`SceneComponent.K2_GetComponentRotation` (`self.PossessionTarget`))) 500.0)) :`ObjectTypes` (`self.eligiblePossTarget`) :`bTraceComplex` true :`DrawDebugType` "Persistent"))
  (bind _output_get (set `self.possTraceHit?` _returnvalue_2))
  (if _output_get
    (bind _output_get_2 (set `self.Is Possessing?` true))
    (bind _output_get_3 (set `self.possHits` _outhits))
    (bind _output (`|GetArrayItem` _output_get_3))
    (bind (_bblockinghit _binitialoverlap _time _distance _location _impactpoint _normal _impactnormal _physmat _hitactor) (`GameplayStatics.BreakHitResult` _output))
    (bind _output_get_4 (set `self.possessedTarget` _hitactor))
    (`self.K2_SetActorLocationAndRotation` self (+ (`self.K2_GetActorLocation` _output_get_4) (0.0 0.0 10.0)) (`self.K2_GetActorRotation` _output_get_4) false false)
    (`self.K2_DestroyActor` _output_get_4))
  (return _output_get_4 _output_get_2 (`GameplayStatics.GetObjectClass` _hitactor) _output_get_3 _output))

(fn `UserConstructionScript`
  (`parent.UserConstructionScript`))

(fn `WindBlast`
  (bind _returnvalue (`self.K2_GetActorLocation`))
  (`GameplayStatics.PlaySound2D` "/Game/Audio/windsurge_001.windsurge_001" 1.0 1.0 0.0 null null)
  (if (`self.hasMana`)
    (bind _outhit (`KismetSystemLibrary.LineTraceSingle` _returnvalue (+ _returnvalue (* (`KismetMathLibrary.GetForwardVector` (`self.GetControlRotation`)) (`KismetMathLibrary.Conv_DoubleToVector` 15000.0))) "TraceTypeQuery1"))
    (if (`self.bWindBlastUpgrade`)
      (bind (_bblockinghit _binitialoverlap _time _distance _location _impactpoint _normal _impactnormal _physmat _hitactor _hitcomponent) (`GameplayStatics.BreakHitResult` _outhit))
      (`PrimitiveComponent.AddImpulse` _hitcomponent (* (`KismetMathLibrary.GetForwardVector` (`self.GetControlRotation`)) (`KismetMathLibrary.Conv_DoubleToVector` 3000.0)) "None" true)
      (else
        (`PrimitiveComponent.AddImpulse` _hitcomponent (* (`KismetMathLibrary.GetForwardVector` (`self.GetControlRotation`)) (`KismetMathLibrary.Conv_DoubleToVector` 1500.0)) "None" true)))
    (bind _returnvalue_2 (`AddComponent|NODE_AddNiagaraComponent-0` :`RelativeTransform` (`SceneComponent.GetRelativeTransform` (`self.FirstPersonCamera`))))
    (`ActorComponent.SetActive` _returnvalue_2 true false)))